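; Networked player pawn for a Mars 2030 VR experience, with a keyboard and mouse fallback.
; Tick initializes it once the HMD is ready, spawning controllers, Vive trackers and HUD.
; Body-capture calibration is saved in the game instance and resent to the server when clients join.
; It also handles teleport, turning, replicated suit lights, drone possession, waypoint paths, photos, dust-storm level streaming and a soft-loaded treadmill component.
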(event Custom|Server%20Set%20Pawn%20Active
  (params (IsPawnActive :type Boolean))
  ;[1 1 1] Set 'IsPawnActive' (replicated)
  (Variables|Default|SetIsPawnActive IsPawnActive))

(event Custom|ServerStartDustStorm
  (Game|LoadStreamLevel(byName) "2045_Events_DustStorm_DGN" true))

(event Custom|Server_RefreshCalibrationForNewClients
  ;[1 1 1] Called for earlier connected players when new player connected
  (bind _outactors (Actor|GetAllActorsOfClass "BP_PlayerPawn_C"))
  (for _array_element _outactors
    (if (Pawn|IsLocallyControlled (.AsBP%20Player%20Pawn (Utilities|Casting|CastToBP_PlayerPawn _array_element)))
      (CallFunction|LocalRefreshCalibrationforNewClients (.AsBP%20Player%20Pawn (Utilities|Casting|CastToBP_PlayerPawn _array_element)))
      (else
        (CallFunction|ClientRefreshCalibrationforNewClients (.AsBP%20Player%20Pawn (Utilities|Casting|CastToBP_PlayerPawn _array_element)))))))

(event Custom|Local_RefreshCalibrationForNewClients
  ;[1 1 1] Resend calibration data to all pawns (because new remote pawns were spawned at newly connected machine)
  (if (Pawn|IsLocallyControlled)
    (Class|CaptureDevice|SendCalibrationtoServer (Variables|Default|GetCaptureDeviceComponent))))

(event Custom|ServerStopDustStorm
  (Game|UnloadStreamLevel(byName) "2045_Events_DustStorm_DGN" false))

(event Custom|Client_RefreshCalibrationForNewClients
  ;[1 1 1] Called for earlier connected players when new player connected
  (CallFunction|LocalRefreshCalibrationforNewClients))

(event Custom|SendNonHMDMove
  ;[1 1 1] Send Non-HMD Moves to Server
  (CallFunction|ServerNonHMDMove (Transformation|GetActorLocation) (Transformation|GetActorRotation)))

(event Custom|PauseMenuNotification
  ;[1 1 1] Pause Menu
  (Class|PauseMenuComponent|TogglePaused (Variables|Default|GetPauseMenuComponent)))

(event Custom|UpdateLightsUsingCurrentState
  ;[1 1 1] Lights
  (switch Utilities|FlowControl|Switch|SwitchonEMissionControlLightState (Class|MissionControlPawn|GetLightState)
    (:Off
      (Rendering|SetVisibility (Variables|Default|GetLWorkLight) false false)
      (Rendering|Material|SetScalarParameterValue (Variables|Default|GetWorkLightMat) "EmissiveStrength" 0.0 :!class /Script/Engine.MaterialInstanceDynamic)
      (Rendering|Material|SetScalarParameterValue (Variables|Default|GetTraverseMat) "EmissiveStrength" 0.0 :!class /Script/Engine.MaterialInstanceDynamic))
    (:WorkOnly
      (Rendering|SetVisibility (Variables|Default|GetLWorkLight) true false)
      (Rendering|SetVisibility (Variables|Default|GetRTraversalLight) false false)
      (Rendering|Material|SetScalarParameterValue (Variables|Default|GetWorkLightMat) "EmissiveStrength" 4e+01 :!class /Script/Engine.MaterialInstanceDynamic)
      (Rendering|Material|SetScalarParameterValue (Variables|Default|GetTraverseMat) "EmissiveStrength" 0.0 :!class /Script/Engine.MaterialInstanceDynamic))
    (:Traversal
      (Rendering|SetVisibility (Variables|Default|GetLWorkLight) true false)
      (Rendering|Material|SetScalarParameterValue (Variables|Default|GetWorkLightMat) "EmissiveStrength" 4e+01 :!class /Script/Engine.MaterialInstanceDynamic)
      (Rendering|Material|SetScalarParameterValue (Variables|Default|GetTraverseMat) "EmissiveStrength" 4e+01 :!class /Script/Engine.MaterialInstanceDynamic))))

(event Custom|OnForceInitialization
  ;[1 1 1] Tick
  ;;[1 1 1] If HMD is connected, enable it and wait until it's ready
  (Variables|Default|SetIsInitialized true)
  (CallFunction|Initialize)
  (Utilities|Time|ClearandInvalidateTimerbyHandle (Variables|Default|GetForceInitializationHandle)))

(event Custom|server_drone
  ;[0.005591 0 0.01562] Enable Drone Mode
  (bind _returnvalue (Game|SpawnActorfromClass "/Game/AdvancedDroneSystem/Blueprints/BP_DronePawn.BP_DronePawn_C" (Math|Transform|MakeTransform (+ (Transformation|GetActorLocation) (Math|Transform|TransformDirection (Transformation|GetActorTransform) "100.000000,0.000000,100.000000")) (Transformation|GetActorRotation) "1.000000,1.000000,1.000000") "AlwaysSpawn" 0 0 0))
  (Pawn|Possess (Pawn|GetController self) _returnvalue))

(event Custom|DoCalibration
  (bind _capturedevicecomponent (Variables|Default|GetCaptureDeviceComponent))
  ;[1 1 1] Calibration
  ;;[1 1 1] Do Calibration
  (Class|CaptureDevice|ToggleCapture _capturedevicecomponent false true)
  (Class|CaptureDevice|Calibrate _capturedevicecomponent)
  (Class|CaptureDevice|ToggleCapture _capturedevicecomponent true false))

(event Custom|BeginCalibrationUX
  ;[1 1 1] Calibration
  ;;[1 1 1] Calibration UX
  (Class|CaptureDevice|ToggleCapture (Variables|Default|GetCaptureDeviceComponent) false false)
  (Rendering|SetVisibility (Variables|Default|GetSkeletalMesh) false true)
  (Rendering|Components|TextRender|SetText (Variables|Default|GetInstructions) (Utilities|Text|ToText(String) (Utilities|String|MakeLiteralString "Calibration: get in T Pose and press calibrate button"))))

(event Custom|FinishCalibrationUX
  ;[1 1 1] Calibration
  ;;[1 1 1] Calibration UX
  (Rendering|SetVisibility (Variables|Default|GetSkeletalMesh) true true)
  (Rendering|Components|TextRender|SetText (Variables|Default|GetInstructions) (Utilities|Text|ToText(String) (Utilities|String|MakeLiteralString)))
  (CallFunction|UpdateLightsUsingCurrentState) ; Make sure lights are in the correct configuration
)

(event Custom|ServerNonHMDMove
  (params (Location :type Vector) (Rotation :type Rotator))
  ;[1 1 1] Send Non-HMD Moves to Server
  (Transformation|SetActorLocationAndRotation Location Rotation))

(event Custom|Initialize
  (bind _capturedevicecomponent (Variables|Default|GetCaptureDeviceComponent))
  ;[1 1 1] Initialization
  (Development|PrintString "Sanity")
  (Utilities|FlowControl|Sequence
    (:then_0
      ;;[1 1 1] Set Tracking Origin
      (switch name (Class|HeadMountedDisplayFunctionLibrary|GetHMDDeviceName)
        (:OculusHMD
          _)
        (:SteamVR
          _))
      (Class|HeadMountedDisplayFunctionLibrary|SetTrackingOrigin "Floor") ; Windows (Oculus / Vive)
    )
    (:then_1
      ;;[1 1 1] Initialize CaptureDevice
      (Class|CaptureDevice|InitializeReferences _capturedevicecomponent (Variables|Default|GetSkeletalMesh))
      (Class|CaptureDevice|UpdateSkeletonSetup _capturedevicecomponent))
    (:then_2
      ;;[1 1 1] Spawn Trackers and Prepare for Calibration
      (if (== (Components|GetOwner) (Game|GetPlayerController 0))
        (Utilities|FlowControl|Sequence
          (:then_0
            (CallFunction|SpawnMotionControllers))
          (:then_1
            (CallFunction|SpawnViveTrackers))
          (:then_2
            (if (Class|HeadMountedDisplayFunctionLibrary|IsHeadMountedDisplayEnabled)
              (CallFunction|InitializeCalibration)
              (else
                (CallFunction|FinishCalibrationUX) ; Skip calibration for KB+M players
              ))))))
    (:then_3
      ;;[1 1 1] Set Base Eye Height
      (if (Class|HeadMountedDisplayFunctionLibrary|IsHeadMountedDisplayEnabled)
        (Variables|Default|SetBaseEyeHeight 0.0)
        (else
          (Variables|Default|SetBaseEyeHeight 165.0))))
    (:then_4
      ;;[1 1 1] Enable/Disable Keyboard Movement
      (Variables|Default|SetEnableKeyboardMovement (not (Class|HeadMountedDisplayFunctionLibrary|IsHeadMountedDisplayEnabled))))
    (:then_5
      (if (Pawn|IsLocallyControlled)
        ;[1 1 1] HUD construction/destruction
        (bind _returnvalue (Game|SpawnActorfromClass "/Game/Mars2030/Blueprints/HUD/BP_HUD.BP_HUD_C" (Math|Transform|MakeTransform "0, 0, 0") "Undefined" 0 0))
        (bind _output_get (Variables|Default|SetHUDActor _returnvalue))
        ;[1 1 1] Attach HUD to camera socket on body in VR
        (Transformation|AttachComponentToComponent _output_get (Variables|Default|GetInformatics) "InformaticsSocket" "SnapToTarget" "SnapToTarget" "SnapToTarget" true)
        (if (Class|HeadMountedDisplayFunctionLibrary|IsHeadMountedDisplayEnabled)
          (Transformation|SetActorRelativeTransform _output_get (Math|Transform|MakeTransform "5.000000,0.000000,25.000000" "0, 0, 0" "3.000000,3.000000,3.000000") false true)
          (else
            (Transformation|SetActorRelativeTransform _output_get (Math|Transform|MakeTransform "0.000000,10.000000,15.000000" "90.000000,90.000000,0.000000") false true)))))))

(event Custom|ExecuteTeleportation
  (params (MotionController :type BP%20Motion%20Controller%20Object%20Reference))
  (bind (_location _rotation) (Default|GetTeleportDestination MotionController))
  ;[1 1 1] Teleport Action
  (if (not (Variables|Default|GetIsTeleporting))
    (if (Variables|/Game/VirtualRealityBP/Blueprints/BP_MotionController.BP_MotionController_C|GetIsValidTeleportDestination MotionController)
      (Variables|Default|SetIsTeleporting true)
      (Default|DisableTeleporter MotionController)
      (Transformation|SetActorLocationAndRotation _location _rotation false true)
      (CallFunction|ServerTeleport _location _rotation)
      (Variables|Default|SetIsTeleporting false)
      (else
        (Default|DisableTeleporter MotionController)))))

(event Custom|SaveCalibrationData
  (bind _capturedevicecomponent (Variables|Default|GetCaptureDeviceComponent))
  (bind (_outbodycalibration _returnvalue) (Class|CaptureDevice|GetCurrentCalibration _capturedevicecomponent))
  ;[1 1 1] Calibration
  ;;[1 1 1] Save Calibration
  (if _returnvalue
    (Default|SavePlayerCalibration (.AsMars%202030%20Game%20Instance (Utilities|Casting|CastToMars2030_GameInstance (Game|GetGameInstance))) _outbodycalibration)))

(event Custom|ResetCalibrationTriggered
  ;[1 1 1] Calibration
  ;;[1 1 1] Trigger Recalibration
  (CallFunction|BeginCalibrationUX))

(event Custom|ServerTeleport
  (params (Location :type Vector) (Rotation :type Rotator))
  ;[1 1 1] Teleport Action
  (Transformation|SetActorLocationAndRotation Location Rotation false true))

(event EventClientPossessed
  (params (NewController :type Controller%20Object%20Reference))
  ;[1 1 1] Possess
  (Development|PrintString "Client_Possessed()" false)
  (Utilities|FlowControl|Sequence
    (:then_0
      (bind _asm2030_player_controller (Utilities|Casting|CastToM2030_PlayerController NewController))
      (EventDispatchers|BindEventtoInvokePauseMenu _asm2030_player_controller (delegate Custom|PauseMenuNotification)))
    (:then_1
      (if (Class|HeadMountedDisplayFunctionLibrary|IsHeadMountedDisplayEnabled)
        (Variables|Default|SetBaseEyeHeight 0.0)
        (else
          (Variables|Default|SetBaseEyeHeight 165.0))))
    (:then_2
      (Utilities|FlowControl|Delay 0.5)
      (CallFunction|ServerRefreshCalibrationforNewClients))))

(event EventPositionPauseMenu
  (params (PauseMenu :type Actor%20Object%20Reference))
  (bind _asbp_pause_screen (Utilities|Casting|CastToBP_PauseScreen PauseMenu))
  (bind _firstpersoncameracomponent (Variables|Default|GetFirstPersonCameraComponent))
  ;[1 1 1] Position Pause Menu
  (Transformation|SetActorLocation _asbp_pause_screen (Transformation|GetWorldLocation _firstpersoncameracomponent) false false)
  (Transformation|SetWorldRotation (Variables|/Game/Mars2030/Blueprints/HUD/BP_PauseScreen.BP_PauseScreen_C|GetDefaultSceneRoot _asbp_pause_screen) (Math|Rotator|MakeRotator 0.0 0.0 (- (.Yaw (Math|Rotator|BreakRotator (Transformation|GetWorldRotation _firstpersoncameracomponent))) 1.8e+02)) false false)
  (Transformation|AddActorLocalOffset _asbp_pause_screen "-125.000000,-75.000000,0.000000" false false)
  (Transformation|SetActorScale3D _asbp_pause_screen "0.090000,0.090000,0.090000"))

(event EventTick
  (params (DeltaSeconds :type Float%20%28single-precision%29))
  (bind _outtrackeddeviceids (Class|SteamVRFunctionLibrary|GetValidTrackedDeviceIds "Controller"))
  (bind _outtrackeddeviceids_2 (Class|SteamVRFunctionLibrary|GetValidTrackedDeviceIds "Other"))
  (bind _returnvalue (Class|HeadMountedDisplayFunctionLibrary|IsHeadMountedDisplayConnected))
  (bind _capturedevicecomponent (Variables|Default|GetCaptureDeviceComponent))
  (bind _vrbodydirection (Variables|Default|GetVRBodyDirection))
  (bind _forceinitializationtimerduration (Variables|Default|GetForceInitializationTImerDuration))
  (bind _returnvalue_2 (Utilities|Array|Length _outtrackeddeviceids))
  (bind _returnvalue_3 (Utilities|Array|Length _outtrackeddeviceids_2))
  (bind _returnvalue_4 (Math|Vector|CrossProduct "0, 0,1.000000" _vrbodydirection))
  (bind _numexpectedtrackers (Variables|/Script/ViveMocapKit.CaptureDevice|GetNumExpectedTrackers _capturedevicecomponent))
  (bind _returnvalue_5 (Math|Rotator|MakeRotationfromAxes _vrbodydirection _returnvalue_4 "0, 0,1.000000"))
  ;[1 1 1] Tick
  (if (Variables|Default|GetIsInitialized)
    (if (and (Pawn|IsLocallyControlled) (Class|HeadMountedDisplayFunctionLibrary|IsHeadMountedDisplayEnabled))
      (Utilities|FlowControl|Sequence
        (:then_1
          (Transformation|SetWorldRotation (Variables|Default|GetUI) _returnvalue_5 false false)
          (Transformation|SetWorldRotation (Variables|/Script/Engine.Actor|GetRootComponent (Variables|Default|GetHUDActor)) _returnvalue_5 false false))
        (:then_2
          ;;[1 1 1] Display tracking stats
          (if (== _numexpectedtrackers 0)
            (if (< _returnvalue_2 2)
              (Rendering|Components|TextRender|SetText (Variables|Default|GetWarning) (Utilities|Text|ToText(String) (Utilities|String|Append "Warning - missing conrollers (got " (Utilities|String|ToString(Integer) _returnvalue_2) "/2)")))
              (elif (and (Class|CaptureDevice|AreHandsSwapped _capturedevicecomponent) (not (Class|CaptureDevice|IsCalibrated _capturedevicecomponent)))
                (Rendering|Components|TextRender|SetText (Variables|Default|GetWarning) (Utilities|Text|MakeLiteralText "Warning - Hand swap detected!"))
                (else
                  (if (< _returnvalue_3 _numexpectedtrackers) :!label _label
                    (Rendering|Components|TextRender|SetText (Variables|Default|GetWarning) (Utilities|Text|ToText(String) (Utilities|String|Append "Warning missing trackers (got " (Utilities|String|ToString(Integer) _returnvalue_3) "/" (Utilities|String|ToString(Integer) _numexpectedtrackers) ")")))
                    (else
                      (Rendering|Components|TextRender|SetText (Variables|Default|GetWarning) (Utilities|Text|MakeLiteralText "")))))))
            (else
              (goto _label))))))
    (else
      ;;[1 1 1] If HMD is connected, enable it and wait until it's ready
      (if _returnvalue
        (Class|HeadMountedDisplayFunctionLibrary|EnableHMD _returnvalue)
        (if (Class|HeadMountedDisplayFunctionLibrary|IsHeadMountedDisplayEnabled) ; Note: don't use return value of EnableHMD as that returns false if stereo is already enabled
          (Variables|Default|SetIsInitialized true :!label _label_2)
          (CallFunction|Initialize)
          (Utilities|Time|ClearandInvalidateTimerbyHandle (Variables|Default|GetForceInitializationHandle))
          (elif (not (and (Utilities|Time|IsValidTimerHandle (Variables|Default|GetForceInitializationHandle)) (!= _forceinitializationtimerduration -1.0)))
            (bind _returnvalue_6 (Utilities|Time|SetTimerbyEvent (EventDispatchers|CreateEvent :!event Custom|OnForceInitialization) _forceinitializationtimerduration))
            (Variables|Default|SetForceInitializationHandle _returnvalue_6)))
        (else
          (goto _label_2))))))

(event EventClientUnPossessed
  (params (OldController :type Controller%20Object%20Reference))
  ;[1 1 1] Possess
  (bind _asm2030_player_controller (Utilities|Casting|CastToM2030_PlayerController OldController))
  (EventDispatchers|UnbindEventfromInvokePauseMenu _asm2030_player_controller (delegate Custom|PauseMenuNotification)))

(event EventOnRepLightState
  ;[1 1 1] Lights
  (switch Utilities|FlowControl|Switch|SwitchonEMissionControlLightState (Class|MissionControlPawn|GetLightState)
    (:Off
      (Rendering|SetVisibility (Variables|Default|GetLWorkLight) false false)
      (Rendering|Material|SetScalarParameterValue (Variables|Default|GetWorkLightMat) "EmissiveStrength" 0.0 :!class /Script/Engine.MaterialInstanceDynamic)
      (Rendering|Material|SetScalarParameterValue (Variables|Default|GetTraverseMat) "EmissiveStrength" 0.0 :!class /Script/Engine.MaterialInstanceDynamic))
    (:WorkOnly
      (Rendering|SetVisibility (Variables|Default|GetLWorkLight) true false)
      (Rendering|SetVisibility (Variables|Default|GetRTraversalLight) false false)
      (Rendering|Material|SetScalarParameterValue (Variables|Default|GetWorkLightMat) "EmissiveStrength" 4e+01 :!class /Script/Engine.MaterialInstanceDynamic)
      (Rendering|Material|SetScalarParameterValue (Variables|Default|GetTraverseMat) "EmissiveStrength" 0.0 :!class /Script/Engine.MaterialInstanceDynamic))
    (:Traversal
      (Rendering|SetVisibility (Variables|Default|GetLWorkLight) true false)
      (Rendering|Material|SetScalarParameterValue (Variables|Default|GetWorkLightMat) "EmissiveStrength" 4e+01 :!class /Script/Engine.MaterialInstanceDynamic)
      (Rendering|Material|SetScalarParameterValue (Variables|Default|GetTraverseMat) "EmissiveStrength" 4e+01 :!class /Script/Engine.MaterialInstanceDynamic))))

(event Input|ActionEvents|InputActionMenuAction
  (params (Key :type Key%20Structure :default "None"))
  ;[1 1 1] Calibration
  ;;[1 1 1] Calibration Input
  (:Pressed
    (if (not (Class|CaptureDevice|IsCapturing (Variables|Default|GetCaptureDeviceComponent)))
      (CallFunction|DoCalibration)
      (if (Class|CaptureDevice|IsCapturing (Variables|Default|GetCaptureDeviceComponent))
        (CallFunction|FinishCalibrationUX)
        (CallFunction|SaveCalibrationData)))))

(event Input|ActionEvents|InputActionMenuAction
  (params (Key :type Key%20Structure :default "None"))
  ;[1 1 1] Calibration
  ;;[1 1 1] Trigger Recalibration
  (:Pressed
    (if (Class|CaptureDevice|IsCapturing (Variables|Default|GetCaptureDeviceComponent))
      (bind _returnvalue (Utilities|Time|SetTimerbyEvent (delegate Custom|ResetCalibrationTriggered) 3.0))
      (Variables|Default|SetResetCalibrationTimer _returnvalue)))
  (:Released
    (Utilities|Time|ClearandInvalidateTimerbyHandle (Variables|Default|GetResetCalibrationTimer))))

(event Input|ActionEvents|InputActionTakePhoto
  (params (Key :type Key%20Structure :default "None"))
  (:Pressed
    (bind _ascamera_2_bp (Utilities|Casting|CastToCamera_2_BP (Variables|/Script/Engine.ChildActorComponent|GetChildActor (Variables|Default|GetCamera_2_BP))))
    (Default|SnapPhoto _ascamera_2_bp)))

(event Input|ActionEvents|InputActionTeleportLeft
  (params (Key :type Key%20Structure :default "None"))
  (bind _leftcontroller (Variables|Default|GetLeftController))
  ;[1 1 1] Teleport Input
  (:Pressed
    (Default|ActivateTeleporter _leftcontroller)
    (Default|DisableTeleporter (Variables|Default|GetRightController)))
  (:Released
    (if (Variables|/Game/VirtualRealityBP/Blueprints/BP_MotionController.BP_MotionController_C|GetIsTeleporterActive _leftcontroller)
      (CallFunction|ExecuteTeleportation _leftcontroller))))

(event Input|ActionEvents|InputActionTeleportRight
  (params (Key :type Key%20Structure :default "None"))
  (bind _rightcontroller (Variables|Default|GetRightController))
  ;[1 1 1] Teleport Input
  (:Pressed
    (Default|ActivateTeleporter _rightcontroller)
    (Default|DisableTeleporter (Variables|Default|GetLeftController)))
  (:Released
    (if (Variables|/Game/VirtualRealityBP/Blueprints/BP_MotionController.BP_MotionController_C|GetIsTeleporterActive _rightcontroller)
      (CallFunction|ExecuteTeleportation _rightcontroller))))

(event Input|ActionEvents|InputActionLightSwitchDown
  (params (Key :type Key%20Structure :default "None"))
  ;[1 1 1] Lights
  (:Pressed
    (Class|MissionControlPawn|SetLightState (Utilities|Select :Index (Class|MissionControlPawn|GetLightState) :Off "Off" :WorkOnly "Off" :Traversal "WorkOnly"))))

(event Input|ActionEvents|InputActionLightSwitchUp
  (params (Key :type Key%20Structure :default "None"))
  ;[1 1 1] Lights
  (:Pressed
    (Class|MissionControlPawn|SetLightState (Utilities|Select :Index (Class|MissionControlPawn|GetLightState) :Off "WorkOnly" :WorkOnly "Traversal" :Traversal "Traversal"))))

(event Input|ActionEvents|InputActionRightToolDpadUp
  (params (Key :type Key%20Structure :default "None"))
  (bind _returnvalue (Transformation|GetActorTransform))
  ;[1 1 1] Inject treadmill
  ;;[1 0.3038 0.2378] Perhaps we can bind this differently, but at least it removes the hard refs
  (:Pressed
    (Default|CallTreadmillButtonDown)
    (CallFunction|ServerTeleport (.location _returnvalue) (.rotation _returnvalue) :!label _label))
  (:Released
    (Default|CallTreadmillButtonUp)
    (goto _label)))

(event Input|ActionEvents|InputActionResponseL
  (params (Key :type Key%20Structure :default "None")))

(event Input|ActionEvents|InputActionResponseR
  (params (Key :type Key%20Structure :default "None")))

(event Input|ActionEvents|InputActionToggleTreadmill
  (params (Key :type Key%20Structure :default "None"))
  (bind _treadmillcomponentclass (Variables|Default|GetTreadmillComponentClass))
  ;[1 1 1] Inject treadmill
  (:Pressed
    (if (Utilities|IsValidSoftClassReference _treadmillcomponentclass) ; Future will be loaded from the plugin which may not be loaded
      (Utilities|FlowControl|FlipFlop
        (:A
          (bind _returnvalue (Utilities|LoadClassAssetBlocking _treadmillcomponentclass))
          (bind _asactor_component (Utilities|Casting|CastToActorComponentClass _returnvalue))
          (bind _returnvalue_2 (Game|AddComponentbyClass _asactor_component)) ; Only for client side
          (Variables|Default|SetTreadmillComponent _returnvalue_2))
        (:B
          (Utilities|IsValid (Variables|Default|GetTreadmillComponent)
            (:Is%20Valid
              (Components|DestroyComponent (Variables|Default|GetTreadmillComponent)))))))))

(event Input|AxisEvents|InputAxisTurn
  (params (AxisValue :type Float%20%28single-precision%29))
  ;[1 1 1] Non-HMD Mouse Camera Rotation
  (if (not (Class|HeadMountedDisplayFunctionLibrary|IsHeadMountedDisplayEnabled))
    (Pawn|Input|AddControllerYawInput AxisValue)
    (Transformation|AddActorLocalRotation (Math|Conversions|RotationFromXVector (Class|KismetMathLibrary|CreateVectorfromYawPitch (* AxisValue (Class|PlayerController|GetDeprecatedInputYawScale (Game|GetPlayerController 0))) 0.0 1.0)) false false)
    (CallFunction|SendNonHMDMove)))

(event Input|AxisEvents|InputAxisMoveForward
  (params (AxisValue :type Float%20%28single-precision%29))
  ;[1 1 1] Keyboard Movement
  (if (and (Variables|Default|GetEnableKeyboardMovement) (!= 0.0 AxisValue))
    (Transformation|AddActorWorldOffset (* (* (Math|Vector|GetForwardVector (Math|Rotator|MakeRotator 0.0 0.0 (.Yaw (Math|Rotator|BreakRotator (Pawn|GetControlRotation :!class /Script/Engine.Pawn))))) AxisValue) (Variables|Default|GetKeyboardMovementSpeed)))
    (CallFunction|SendNonHMDMove)))

(event Input|AxisEvents|InputAxisLookUp
  (params (AxisValue :type Float%20%28single-precision%29))
  ;[1 1 1] Non-HMD Mouse Camera Rotation
  (if (not (Class|HeadMountedDisplayFunctionLibrary|IsHeadMountedDisplayEnabled))
    (Pawn|Input|AddControllerPitchInput AxisValue)))

(event Input|AxisEvents|InputAxisTurnRate
  (params (AxisValue :type Float%20%28single-precision%29))
  (bind _snap_rotation_degrees (Variables|Default|GetSnap%20Rotation%20Degrees))
  ;[1 1 1] Smooth Rotation
  (Utilities|FlowControl|Delay 0.1)
  (if (Variables|Default|Getbsmooth_rotation)
    (if true
      (Transformation|SetActorRotation (Math|Rotator|MakeRotator 0.0 0.0 (+ (.yaw (Transformation|GetActorRotation)) (* AxisValue (Variables|Default|GetSmoothRotationSpeed))))))
    (elif (> (Math|Float|Absolute(Float) AxisValue) (Variables|Default|Getturndeadzone))
      (if (> AxisValue 0.0)
        (Variables|Default|SetRotation%20Angle _snap_rotation_degrees)
        (else
          (Variables|Default|SetRotation%20Angle (- -1.0 _snap_rotation_degrees))))
      (Utilities|FlowControl|DoOnce false :!label _label
        (:Completed
          (Utilities|FlowControl|Sequence
            (:then_0
              (Transformation|SetActorRotation (Math|Rotator|MakeRotator 0.0 0.0 (+ (.yaw (Transformation|GetActorRotation)) (Variables|Default|GetRotation%20Angle)))))
            (:then_1
              (Utilities|FlowControl|Delay 0.2)
              (goto _label Reset)))))
      (else
        (goto _label Reset)))))

(event Input|AxisEvents|InputAxisMoveRight
  (params (AxisValue :type Float%20%28single-precision%29))
  ;[1 1 1] Keyboard Movement
  (if (and (Variables|Default|GetEnableKeyboardMovement) (!= 0.0 AxisValue))
    (Transformation|AddActorWorldOffset (* (* (Math|Vector|GetRightVector (Math|Rotator|MakeRotator 0.0 0.0 (.Yaw (Math|Rotator|BreakRotator (Pawn|GetControlRotation :!class /Script/Engine.Pawn))))) AxisValue) (Variables|Default|GetKeyboardMovementSpeed)))
    (CallFunction|SendNonHMDMove)))

(event Input|KeyboardEvents|G
  (params (Key :type Key%20Structure :default "None")))

(event Input|KeyboardEvents|L
  (params (Key :type Key%20Structure :default "None"))
  (:Pressed
    (CallFunction|FindPathtoActor)))

(event Input|KeyboardEvents|V
  (params (Key :type Key%20Structure :default "None"))
  ;[0.005591 0 0.01562] Enable Drone Mode
  (:Pressed
    (if (Pawn|IsLocallyControlled)
      (CallFunction|ServerDrone))))

(event Input|KeyboardEvents|8
  (params (Key :type Key%20Structure :default "None"))
  (:Pressed
    (CallFunction|ServerStartDustStorm)))

(event Input|KeyboardEvents|9
  (params (Key :type Key%20Structure :default "None"))
  (:Pressed
    (CallFunction|ServerStopDustStorm)))

(event Input|KeyboardEvents|R
  (params (Key :type Key%20Structure :default "None")))

(fn ConstructionScript
  (Transformation|SetWorldLocation (Variables|Default|GetFirstPersonCameraComponent) (Transformation|GetSocketLocation (Variables|Default|GetSkeletalMesh) "HeadSocket") false false)
  ;[1 1 1] Setup Lights
  (Utilities|FlowControl|Sequence
    (:then_0
      (bind _returnvalue (Rendering|Material|CreateDynamicMaterialInstance (Variables|Default|GetRightWorkLight) 0 "/Game/XemuSuit/INFORMATICS/M_InfoLight.M_InfoLight" "None" :!class /Script/Engine.PrimitiveComponent))
      (bind _output_get (Variables|Default|SetWorkLightMat _returnvalue))
      (Rendering|Material|SetMaterial (Variables|Default|GetLeftWorkLight) 0 _output_get))
    (:then_1
      (bind _returnvalue_2 (Rendering|Material|CreateDynamicMaterialInstance (Variables|Default|GetRightTraversalLight) 0 "/Game/XemuSuit/INFORMATICS/M_InfoLight.M_InfoLight" "None" :!class /Script/Engine.PrimitiveComponent))
      (bind _output_get_2 (Variables|Default|SetTraverseMat _returnvalue_2))
      (Rendering|Material|SetMaterial (Variables|Default|GetLeftTraversalLight) 0 _output_get_2))))

(fn SpawnViveTrackers
  ;[1 1 1] Add Motion Controllers for Vive Trackers
  (for _array_element (Utilities|Array|MakeArray 1 2 3 4 5)
    (bind _returnvalue (AddComponent|AddMotionControllerComponent false (Math|Transform|MakeTransform "0, 0, 0")))
    (Transformation|AttachComponentToComponent _returnvalue (Variables|Default|GetScene1) "None" "SnapToTarget" "SnapToTarget" "KeepWorld" false)
    (Variables|/Script/HeadMountedDisplay.MotionControllerComponent|SetMotionSource _returnvalue (Utilities|String|StringToName (Utilities|String|Append "Special_" (Utilities|String|ToString(Integer) _array_element))))
    (Variables|/Script/HeadMountedDisplay.MotionControllerComponent|SetDisplayModelSource _returnvalue "SteamVR")
    (Variables|/Script/HeadMountedDisplay.MotionControllerComponent|SetbDisplayDeviceModel _returnvalue false)))

(fn SpawnMotionControllers
  (bind _returnvalue (Math|Transform|MakeTransform "0, 0, 0"))
  (bind _self self)
  (Utilities|FlowControl|Sequence
    (:then_0
      ;[1 1 1] Spawn Left Controller
      (bind _returnvalue_2 (Game|SpawnActorfromClass "/Game/VirtualRealityBP/Blueprints/BP_MotionController.BP_MotionController_C" _returnvalue "AlwaysSpawn" _self "Left" 0)) ; "Hand" is available by checking "Expose on Spawn in the variable on BP_MotionController.
      (bind _output_get (Variables|Default|SetLeftController _returnvalue_2))
      (Transformation|AttachComponentToComponent _output_get (Variables|Default|GetScene1) "None" "SnapToTarget" "SnapToTarget" "KeepWorld" false))
    (:then_1
      ;[1 1 1] Spawn Right Controller
      (bind _returnvalue_3 (Game|SpawnActorfromClass "/Game/VirtualRealityBP/Blueprints/BP_MotionController.BP_MotionController_C" _returnvalue "AlwaysSpawn" _self "Right" 0)) ; "Hand" is available by checking "Expose on Spawn in the variable on BP_MotionController.
      (bind _output_get_2 (Variables|Default|SetRightController _returnvalue_3))
      (Transformation|AttachComponentToComponent _output_get_2 (Variables|Default|GetScene1) "None" "SnapToTarget" "SnapToTarget" "KeepWorld" false))))

(fn InitializeCalibration
  (bind _capturedevicecomponent (Variables|Default|GetCaptureDeviceComponent))
  (bind _asmars_2030_game_instance (Utilities|Casting|CastToMars2030_GameInstance (Game|GetGameInstance))
    (:then
      (bind (_success _calibration) (Default|GetPlayerCalibration _asmars_2030_game_instance)) ; Check for existing calibration data
      (if _success
        ;[1 1 1] Use existing calibration data
        (Class|CaptureDevice|ApplyCurrentCalibration _capturedevicecomponent _calibration)
        (Class|CaptureDevice|ToggleCapture _capturedevicecomponent true true)
        (Class|CaptureDevice|SendCalibrationtoServer _capturedevicecomponent)
        (else
          (CallFunction|BeginCalibrationUX :!label _label) ; Prompt player to calibrate
        )))
    (:CastFailed
      (Development|PrintString "Cast Failed (Mars2030_GameModeInstance)" true true "(R=1.000000,G=0.000000,B=0.004727,A=1.000000)" 1e+01)
      (goto _label))))

(fn OnRepIsPawnActive
  (bind _ispawnactive (Variables|Default|GetIsPawnActive))
  (Collision|SetActorEnableCollision _ispawnactive)
  (Rendering|SetActorHiddenInGame (not _ispawnactive)))

(fn FindPathtoActor
  (bind _objectiveactor (Variables|Default|GetObjectiveActor))
  (Utilities|IsValid _objectiveactor
    (:Is%20Valid
      (Variables|Default|SetblsFindPathtoActor true)
      (Default|FindPathtoActor (Variables|Default|GetBP_WaypointComponent) _objectiveactor (Variables|Default|GetSpline)))))

(fn FinishPathFinding
  (Default|FinishFindingWaypoint (Variables|Default|GetBP_WaypointComponent)))

(fn GetHandManager
  (return 0))
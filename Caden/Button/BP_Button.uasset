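; BP_Button is a pressure button that raises a referenced actor when something holds it down.
; Each Tick, overlaps on the Box step the mesh down within ButtonOffset, and it steps back up when clear.
; Near the bottom it lifts the Actor, then disables Box collision for a two-second cooldown and prints debug state throughout.
; The construction script sets the arrow length and mesh rest height from ButtonOffset.
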(event EventTick
  (params (DeltaSeconds :type Float%20%28single-precision%29))
  (bind _staticmesh (Variables|Default|GetStaticMesh))
  (bind _staticmesh_2 (Variables|Default|GetStaticMesh))
  (bind _box (Variables|Default|GetBox))
  (bind _staticmesh_3 (Variables|Default|GetStaticMesh))
  (bind _actor (Variables|Default|GetActor))
  (bind _returnvalue (Transformation|GetActorLocation _actor))
  (bind _relativelocation (Variables|/Script/Engine.SceneComponent|GetRelativeLocation _staticmesh_2))
  (Variables|Default|SetIspressed (<= (.z _relativelocation) 1e+01))
  (Development|PrintString (Utilities|String|ToString(Text) (Utilities|Text|FormatText "{box} is pressed:{ispressed} " (Math|Float|Truncate (.z _relativelocation)) (Variables|Default|GetIspressed))))
  (if (> (Utilities|Array|Length (Collision|GetOverlappingActors (Variables|Default|GetBox) 0 :!class /Script/Engine.PrimitiveComponent)) 0)
    (Components|MoveComponentTo _staticmesh_3 (Math|Vector|MakeVector 0.0 0.0 (Math|Float|Clamp(Float) (- (.z (Variables|/Script/Engine.SceneComponent|GetRelativeLocation _staticmesh_3)) 3.0) 0.0 (Variables|Default|GetButtonOffset))) "0, 0, 0" false false 0.01 false)
    (if (Variables|Default|GetIspressed)
      (Transformation|SetActorLocation _actor (Math|Vector|MakeVector (.x _returnvalue) (.y _returnvalue) (+ (.z _returnvalue) 1e+01)) false false)
      (Collision|SetCollisionEnabled _box "NoCollision")
      (Utilities|FlowControl|Delay 2.0)
      (Collision|SetCollisionEnabled _box "QueryAndPhysics"))
    (else
      (Components|MoveComponentTo _staticmesh (Math|Vector|MakeVector 0.0 0.0 (Math|Float|Clamp(Float) (+ (.z (Variables|/Script/Engine.SceneComponent|GetRelativeLocation _staticmesh)) 3.0) 0.0 (Variables|Default|GetButtonOffset))) "0, 0, 0" false false 0.01 false))))

(fn ConstructionScript
  (bind _buttonoffset (Variables|Default|GetButtonOffset))
  (Variables|/Script/Engine.ArrowComponent|SetArrowLength (Variables|Default|GetArrow) _buttonoffset)
  (Transformation|SetRelativeLocation (Variables|Default|GetStaticMesh) (Math|Vector|MakeVector 0.0 0.0 _buttonoffset) false false))
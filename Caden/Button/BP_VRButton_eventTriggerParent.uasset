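; VR push-button Blueprint that triggers a Possessdrone call when pressed, apparently as a parent for event-triggering buttons.
; Each Tick, actors overlapping the Box sink the mesh in small clamped steps, and it rises back toward ButtonOffset once clear.
; Reaching the height threshold while overlapped fires the call, then briefly disables Box collision as a cooldown.
; The construction script sets the arrow length and resting mesh height from ButtonOffset.
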(event OnComponentBeginOverlap(Box)
  (params (OverlappedComponent :type Primitive%20Component%20Object%20Reference) (OtherActor :type Actor%20Object%20Reference) (OtherComp :type Primitive%20Component%20Object%20Reference) (OtherBodyIndex :type Integer) (bFromSweep :type Boolean) (SweepResult :type Hit%20Result%20Structure%20%28by%20ref%29)))

(event EventTick
  (params (DeltaSeconds :type Float%20%28single-precision%29))
  (bind _staticmesh (Variables|Default|GetStaticMesh))
  (bind _staticmesh_2 (Variables|Default|GetStaticMesh))
  (bind _box (Variables|Default|GetBox))
  (Variables|Default|SetIspressed (<= (.z (Variables|/Script/Engine.SceneComponent|GetRelativeLocation (Variables|Default|GetStaticMesh))) 2e+01))
  (if (> (Utilities|Array|Length (Collision|GetOverlappingActors (Variables|Default|GetBox) 0 :!class /Script/Engine.PrimitiveComponent)) 0)
    (Components|MoveComponentTo _staticmesh_2 (Math|Vector|MakeVector 0.0 0.0 (Math|Float|Clamp(Float) (- (.z (Variables|/Script/Engine.SceneComponent|GetRelativeLocation _staticmesh_2)) 3.0) 0.0 (Variables|Default|GetButtonOffset))) "0, 0, 0" false false 0.01 false)
    (if (Variables|Default|GetIspressed)
      (Default|CallPossessdrone)
      (Collision|SetCollisionEnabled _box "NoCollision")
      (Utilities|FlowControl|Delay 2.0)
      (Collision|SetCollisionEnabled _box "QueryAndPhysics"))
    (else
      (Components|MoveComponentTo _staticmesh (Math|Vector|MakeVector 0.0 0.0 (Math|Float|Clamp(Float) (+ (.z (Variables|/Script/Engine.SceneComponent|GetRelativeLocation _staticmesh)) 3.0) 0.0 (Variables|Default|GetButtonOffset))) "0, 0, 0" false false 0.01 false))))

(fn ConstructionScript
  (bind _buttonoffset (Variables|Default|GetButtonOffset))
  (Variables|/Script/Engine.ArrowComponent|SetArrowLength (Variables|Default|GetArrow) _buttonoffset)
  (Transformation|SetRelativeLocation (Variables|Default|GetStaticMesh) (Math|Vector|MakeVector 0.0 0.0 _buttonoffset) false false))
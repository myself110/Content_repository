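; BP_StartMenu is an actor with a sphere, text label and widget that can dissolve away on demand.
; Each tick, the label and widget show and turn toward player 0's pawn when it is near, and hide otherwise.
; The construction script sets the label from ObjectName.
; StartDissolve plays a fade sound and a timeline driving the sphere material's Dissolve parameter, with a delayed destroy triggered from the timeline's Update.
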(event Custom|StartDissolve
  (Audio|PlaySound2D "/Game/Caden/FadeEffect/FX_Fade.FX_Fade" 1.0 1.0 0.0 0 0)
  (bind _dissolvetime (Timeline|Timeline_0 Play)
    (:Update
      (Rendering|Material|SetScalarParameterValueonMaterials (Variables|Default|GetSphere) "Dissolve" _dissolvetime)
      (Utilities|FlowControl|Delay 1.0)
      (Actor|DestroyActor))))

(event EventTick
  (params (DeltaSeconds :type Float%20%28single-precision%29))
  (bind _textrender (Variables|Default|GetTextRender))
  ;[1 1 1] Text render and face to pawn
  (if (< (Math|Vector|VectorLength (- (Transformation|GetActorLocation (Game|Player|GetPlayerPawn 0)) (Transformation|GetActorLocation))) 5e+02)
    (Rendering|SetVisibility _textrender true false)
    (Transformation|SetWorldRotation (Variables|Default|GetTextRender) (Math|Rotator|FindLookatRotation (Transformation|GetActorLocation) (Transformation|GetActorLocation (Game|Player|GetPlayerPawn 0))) false false)
    (else
      (Rendering|SetVisibility _textrender false false))))

(fn ConstructionScript
  (Rendering|Components|TextRender|SetText (Variables|Default|GetTextRender) (Variables|Default|GetObjectName)))
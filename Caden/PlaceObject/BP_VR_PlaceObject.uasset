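; VR pawn that moves by axis input and places a BP_TpObject where the right motion controller aims.
; While TeleportRight is held, Tick predicts a projectile arc from the controller, stores the hit location and draws a debug cylinder there.
; Releasing spawns the object at the last stored location instead of teleporting the pawn.
; CanTeleport is computed from the surface normal but does not gate spawning; actual teleport code is disconnected.
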(event EventBeginPlay
  ;[1 1 1] left hand setting
  (Transformation|SetWorldScale3D (Variables|Default|GetLeftHand) "1.000000,1.000000,-1.000000"))

(event EventTick
  (params (DeltaSeconds :type Float%20%28single-precision%29))
  (if (Variables|Default|GetTeleportKeyPress)
    (CallFunction|TraceforTeleportation)))

(event Input|ActionEvents|InputActionTeleportLeft
  (params (Key :type Key%20Structure :default "None")))

(event Input|ActionEvents|InputActionTeleportRight
  (params (Key :type Key%20Structure :default "None"))
  (:Pressed
    (Variables|Default|SetTeleportKeyPress true))
  (:Released
    (Variables|Default|SetTeleportKeyPress false)
    (Development|PrintString "teleport")
    (bind _returnvalue (Game|SpawnActorfromClass "/Game/Caden/PlaceObject/BP_TpObject.BP_TpObject_C" (Math|Conversions|ToTransform(Vector) (Variables|Default|GetTPLocation)) "Undefined" 0 0))
    (Development|PrintString (Utilities|GetDisplayName _returnvalue))))

(event Input|AxisEvents|InputAxisOmniVehicleDirectionY
  (params (AxisValue :type Float%20%28single-precision%29))
  (bind _defaultsceneroot (Variables|Default|GetDefaultSceneRoot))
  (bind _returnvalue (Math|Vector|GetForwardVector _defaultsceneroot))
  ;[1 1 1] Movement
  (Pawn|Input|AddMovementInput (Math|Vector|MakeVector (.x _returnvalue) (.y _returnvalue) 0.0) (* AxisValue -1.0) false))

(event Input|AxisEvents|InputAxisOmniVehicleDirectionX
  (params (AxisValue :type Float%20%28single-precision%29))
  (bind _defaultsceneroot (Variables|Default|GetDefaultSceneRoot))
  (bind _returnvalue (Math|Vector|GetRightVector _defaultsceneroot))
  ;[1 1 1] Movement
  (Pawn|Input|AddMovementInput (Math|Vector|MakeVector (.x _returnvalue) (.y _returnvalue) 0.0) (* AxisValue 1.0) false))

(fn ConstructionScript)

(fn TraceforTeleportation
  (bind _rightmc (Variables|Default|GetRightMC))
  (bind (_outhit _outpathpositions _outlasttracedestination _returnvalue) (Class|GameplayStatics|BlueprintPredictProjectilePathbyObjectType (Transformation|GetWorldLocation _rightmc) (* (Math|Vector|GetForwardVector (Transformation|GetWorldRotation _rightmc)) (Variables|Default|GetTeleportationTraceLength)) true 5.0 (Utilities|Array|MakeArray "ObjectTypeQuery1" "ObjectTypeQuery2") false 0 "ForOneFrame" 0.0 15.0 2.0 -5e+02))
  (if _returnvalue
    (Variables|Default|SetTPLocation (.Location (Collision|BreakHitResult _outhit)))
    (Development|PrintString (Utilities|String|ToString(Float) (.Z (Math|Vector|BreakVector (.ImpactNormal (Collision|BreakHitResult _outhit))))))
    (LocalVariables|SetCanTeleport (> (.Z (Math|Vector|BreakVector (.ImpactNormal (Collision|BreakHitResult _outhit)))) 0.0))
    (bind _output_get (Variables|Default|SetTeleportLocation (.ImpactPoint (Collision|BreakHitResult _outhit))))
    (Class|KismetSystemLibrary|DrawDebugCylinder _output_get (+ _output_get "0,0,20.000000") 5e+01 20 "(R=0.150525,G=0.000000,B=1.000000,A=1.000000)" 0.0 0.0)))
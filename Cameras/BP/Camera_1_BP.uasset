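; Placeable camera actor that feeds a scene capture into one render target slot of a CameraSystem monitor.
; Two seconds after BeginPlay, it finds CameraSystem actors whose ScreenID matches Monitor, assigns the capture's texture target by Position, then destroys its Camera component.
; The construction script applies mesh choice, rotation, pitch, capture rate and lens material settings, and mirrors FOV between the Camera and scene capture.
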(event EventBeginPlay
  (bind _oooooooo (Variables|Default|Getoooooooo))
  (bind _outactors (Actor|GetAllActorsOfClass "/Game/Cameras/BP/CameraSystem.CameraSystem_C"))
  (Utilities|FlowControl|Delay 2.0)
  (for _array_element _outactors
    (if (== (Variables|/Game/Cameras/BP/CameraSystem.CameraSystem_C|GetScreenID _array_element) (Variables|Monitor|GetMonitor?))
      (switch int (Variables|Monitor|GetPosition)
        (:0
          (Variables|/Script/Engine.SceneCaptureComponent2D|SetTextureTarget _oooooooo (Variables|/Game/Cameras/BP/CameraSystem.CameraSystem_C|GetRender1 _array_element)))
        (:1
          (Variables|/Script/Engine.SceneCaptureComponent2D|SetTextureTarget _oooooooo (Variables|/Game/Cameras/BP/CameraSystem.CameraSystem_C|GetRender2 _array_element)))
        (:2
          (Variables|/Script/Engine.SceneCaptureComponent2D|SetTextureTarget _oooooooo (Variables|/Game/Cameras/BP/CameraSystem.CameraSystem_C|GetRender3 _array_element)))
        (:3
          (Variables|/Script/Engine.SceneCaptureComponent2D|SetTextureTarget _oooooooo (Variables|/Game/Cameras/BP/CameraSystem.CameraSystem_C|GetRender4 _array_element))))))
  (Components|DestroyComponent (Variables|Default|GetCamera)))

(fn ConstructionScript
  (bind _camera (Variables|Default|GetCamera))
  (bind _oooooooo (Variables|Default|Getoooooooo))
  (bind _rotation (Variables|CameraSettings|GetRotation))
  (bind _1 (Variables|Default|Get1))
  (bind _fov (Variables|CameraSettings|GetFOV))
  (bind _relativerotation (Variables|/Script/Engine.SceneComponent|GetRelativeRotation _camera))
  (bind (_roll _pitch _yaw) (Math|Rotator|BreakRotator _relativerotation))
  (bind _returnvalue (Rendering|Material|CreateDynamicMaterialInstance (Variables|Default|Get1) 1 "/Game/Cameras/Material/Camera1_Inst.Camera1_Inst" "None" :!class /Script/Engine.PrimitiveComponent))
  (Rendering|Material|SetScalarParameterValueonMaterials (Variables|Default|Get1) "Rotation" _rotation)
  (Transformation|SetWorldRotation (Variables|Default|GetSphere) (Math|Rotator|MakeRotator 0.0 0.0 (Math|Float|MapRangeUnclamped _rotation 0.0 1.0 0.0 3.6e+02)) false false)
  (Variables|/Script/Engine.CameraComponent|SetFieldOfView (Variables|Default|GetCamera) _fov)
  (Variables|/Script/Engine.SceneCaptureComponent2D|SetFOVAngle _oooooooo _fov)
  (Transformation|SetRelativeRotation _camera (Math|Rotator|MakeRotator _roll (+ _pitch (Variables|CameraSettings|GetPitch)) _yaw) false false)
  (Variables|/Script/Engine.SceneCaptureComponent|SetbCaptureEveryFrame _oooooooo (Variables|CameraSettings|GetCaptureEveryFrame?))
  (Rendering|Material|SetVectorParameterValue _returnvalue "LenseColor" (Variables|CameraSettings|GetLenseColor) :!class /Script/Engine.MaterialInstanceDynamic)
  (Rendering|Material|SetScalarParameterValue _returnvalue "LenseBrightness" (Variables|CameraSettings|GetLenseBrightness) :!class /Script/Engine.MaterialInstanceDynamic)
  (if (Variables|CameraSettings|GetCameraMesh)
    (Components|StaticMesh|SetStaticMesh _1 "/Game/Cameras/Mesh/2.2")
    (else
      (Components|StaticMesh|SetStaticMesh _1 "/Game/Cameras/Mesh/1.1"))))
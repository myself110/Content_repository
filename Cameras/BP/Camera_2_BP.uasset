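; Security camera actor whose scene capture feeds one of four render targets on the CameraSystem matching its Monitor ID, chosen by Position.
; The link is made two seconds after BeginPlay, then the Camera component is destroyed.
; SnapPhoto uses a temporary capture component copying the main capture's transform and post-process to export a timestamped PNG to the Saved directory.
; The construction script applies FOV, capture frequency, and lens and light material parameters.
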(event Custom|SnapPhoto
  (bind _returnvalue (Math|DateTime|UTCNow))
  (bind _oooooooo (Variables|Default|Getoooooooo))
  (Utilities|IsValid (Variables|Default|GetTempPhotoComponent) ; should be one frame after creation
    (:Is%20Not%20Valid
      (bind _returnvalue_2 (AddComponent|AddSceneCaptureComponent2D false (Math|Transform|ComposeTransforms (Transformation|GetWorldTransform _oooooooo) (Math|Transform|InvertTransform (Transformation|GetActorTransform)))))
      (bind _output_get (Variables|Default|SetTempPhotoComponent _returnvalue_2))
      (Variables|/Script/Engine.SceneCaptureComponent2D|SetPostProcessSettings _output_get (Variables|/Script/Engine.SceneCaptureComponent2D|GetPostProcessSettings _oooooooo))
      (Variables|/Script/Engine.SceneCaptureComponent2D|SetTextureTarget _output_get (Variables|Default|GetPictureTarget))
      (Variables|/Script/Engine.SceneCaptureComponent|SetCaptureSource _output_get "SCS_FinalColorLDR")
      (Rendering|SceneCapture|CaptureScene (Variables|Default|GetTempPhotoComponent) :!class /Script/Engine.SceneCaptureComponent2D)
      (Class|ImageWriteBlueprintLibrary|ExporttoDisk (Variables|Default|GetPictureTarget) (Class|BlueprintPathsLibrary|Combine (Utilities|Array|MakeArray (Class|KismetSystemLibrary|GetProjectSavedDirectory) (Utilities|String|ToString(Text) (Utilities|Text|FormatText "{y}-{m}-{d}_{h}-{mm}-{s}.png" (Utilities|Text|ToText(Integer) (Class|KismetMathLibrary|GetYear _returnvalue) false false) (Class|KismetMathLibrary|GetMonth _returnvalue) (Class|KismetMathLibrary|GetDay _returnvalue) (Class|KismetMathLibrary|GetHour _returnvalue) (Class|KismetMathLibrary|GetMinute _returnvalue) (Class|KismetMathLibrary|GetSecond _returnvalue))))) (Utilities|Struct|MakeImageWriteOptions "PNG" (EventDispatchers|CreateEvent :!event Custom|CameraPictureTaken)))
      (Components|DestroyComponent (Variables|Default|GetTempPhotoComponent)))))

(event Custom|CameraPictureTaken
  (params (bSuccess :type Boolean)))

(event EventBeginPlay
  (bind _oooooooo (Variables|Default|Getoooooooo))
  (bind _outactors (Actor|GetAllActorsOfClass "/Game/Cameras/BP/CameraSystem.CameraSystem_C"))
  (Utilities|FlowControl|Delay 2.0)
  (for _array_element _outactors
    (if (== (Variables|/Game/Cameras/BP/CameraSystem.CameraSystem_C|GetScreenID _array_element) (Variables|Monitor|GetMonitor?))
      (switch int (Variables|Monitor|GetPosition)
        (:0
          (Variables|/Script/Engine.SceneCaptureComponent2D|SetTextureTarget _oooooooo (Variables|/Game/Cameras/BP/CameraSystem.CameraSystem_C|GetRender1 _array_element)))
        (:1
          (Variables|/Script/Engine.SceneCaptureComponent2D|SetTextureTarget _oooooooo (Variables|/Game/Cameras/BP/CameraSystem.CameraSystem_C|GetRender2 _array_element)))
        (:2
          (Variables|/Script/Engine.SceneCaptureComponent2D|SetTextureTarget _oooooooo (Variables|/Game/Cameras/BP/CameraSystem.CameraSystem_C|GetRender3 _array_element)))
        (:3
          (Variables|/Script/Engine.SceneCaptureComponent2D|SetTextureTarget _oooooooo (Variables|/Game/Cameras/BP/CameraSystem.CameraSystem_C|GetRender4 _array_element))))))
  (Components|DestroyComponent (Variables|Default|GetCamera)))

(fn ConstructionScript
  (bind _fov (Variables|CameraSettings|GetFOV))
  (bind _oooooooo (Variables|Default|Getoooooooo))
  (Camera|SetFieldOfView (Variables|Default|GetCamera) _fov)
  (Variables|/Script/Engine.SceneCaptureComponent2D|SetFOVAngle _oooooooo _fov)
  (Variables|/Script/Engine.SceneCaptureComponent|SetbCaptureEveryFrame _oooooooo (Variables|CameraSettings|GetCaptureEveryFrame?))
  (bind _returnvalue (Rendering|Material|CreateDynamicMaterialInstance (Variables|Default|GetCamera2_Static_Camera_1_2) 0 "/Game/Cameras/Material/Cam2_Lense_Inst.Cam2_Lense_Inst" "None" :!class /Script/Engine.PrimitiveComponent))
  (Rendering|Material|SetVectorParameterValue _returnvalue "LenseColor" (Variables|CameraSettings|GetLenseColor) :!class /Script/Engine.MaterialInstanceDynamic)
  (Rendering|Material|SetVectorParameterValue _returnvalue "LightColor" (Variables|CameraSettings|GetLightColor) :!class /Script/Engine.MaterialInstanceDynamic)
  (Rendering|Material|SetScalarParameterValue _returnvalue "LenseBrightness" (Variables|CameraSettings|GetLenseBrightness) :!class /Script/Engine.MaterialInstanceDynamic)
  (Rendering|Material|SetScalarParameterValue _returnvalue "LightBrightness" (Variables|CameraSettings|GetLightBrightness) :!class /Script/Engine.MaterialInstanceDynamic))
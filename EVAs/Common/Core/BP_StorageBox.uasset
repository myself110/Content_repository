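; Storage box actor for VR EVAs that lets players browse and take items held by a MissionControlStorageManager.
; Authority-bound, rate-limited switches toggle it open, cycle the class index with wraparound, or spawn the selection at the drop point, close and notify the manager.
; OnReps of index and class refresh a collision-stripped carryable preview, a temporary interface marked as lacking multiplayer support.
; Open status drives menu visibility and debug switch color.
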(event Custom|DebugSetOpen
  (params (DbgIsOpen :type Boolean))
  ;[1 1 1] Check if we can open the box or not
  (if (not DbgIsOpen)
    (Class|MissionControlStorageManager|SetIsOpen (Variables|Default|GetMissionControlStorageManager) DbgIsOpen)))

(event Custom|VRTapLeft
  ;[1 1 1] Run on authority
  (Utilities|DoOnceDelayReset (Variables|Default|GetServerDelayTimeBetweenHits))
  (CallFunction|ServerSetIndex (- (Variables|Default|GetClassIndex) 1)))

(event Custom|VRTapCenter
  ;[1 1 1] Run on authority
  (Utilities|DoOnceDelayReset (Variables|Default|GetServerDelayTimeBetweenHits))
  (Game|SpawnActorfromClass (Variables|Default|GetActiveClass) (Transformation|GetWorldTransform (Variables|Default|GetDropPoint)) "AlwaysSpawn" 0 0)
  (Variables|Default|SetClassIndex 0)
  (Class|MissionControlStorageManager|ServerSetIsOpen (Variables|Default|GetMissionControlStorageManager) false)
  (Utilities|FlowControl|Sequence
    (:then_0
      (bind _asmars_2030carryable_base (Utilities|Casting|CastToMars2030CarryableBaseClass (Variables|Default|GetActiveClass)))
      (Class|MissionControlStorageManager|ServerCollectItem (Variables|Default|GetMissionControlStorageManager) _asmars_2030carryable_base "Left"))
    (:then_1
      (Variables|Default|SetActiveClass 0))))

(event Custom|VRTapRight
  ;[1 1 1] Run on authority
  (Utilities|DoOnceDelayReset (Variables|Default|GetServerDelayTimeBetweenHits))
  (CallFunction|ServerSetIndex (+ (Variables|Default|GetClassIndex) 1)))

(event Custom|LocalUpdateOpenStatus
  (bind _missioncontrolstoragemanager (Variables|Default|GetMissionControlStorageManager))
  (bind _returnvalue (Class|MissionControlStorageManager|GetIsOpen _missioncontrolstoragemanager))
  ;[1 1 1] Update on open status
  (Rendering|Material|SetVectorParameterValue (Variables|Default|GetDebugSwitchMaterial) "Color" (select _returnvalue "(R=0.000000,G=1.000000,B=0.000000,A=1.000000)" "(R=1.000000,G=0.000000,B=0.000000,A=1.000000)") :!class /Script/Engine.MaterialInstanceDynamic)
  (CallFunction|UpdateMenuVisuals _returnvalue))

(event Custom|ServerSetIndex
  (params (NewIndex :type Integer))
  ;[1 1 1] Run on authority
  (bind _clampedindex (CallFunction|ClampIndex NewIndex))
  (bind _output_get (Variables|Default|SetClassIndex _clampedindex))
  (Variables|Default|SetActiveClass (Utilities|Array|Get(acopy) (Class|MissionControlStorageManager|GetStoredObjectClasses (Variables|Default|GetMissionControlStorageManager)) _output_get)))

(event Custom|TapOpenToggle
  (bind _missioncontrolstoragemanager (Variables|Default|GetMissionControlStorageManager))
  (bind _returnvalue (Class|MissionControlStorageManager|GetIsOpen _missioncontrolstoragemanager))
  (bind _returnvalue_2 (not _returnvalue))
  ;[1 1 1] Run on authority
  (Utilities|DoOnceDelayReset (Variables|Default|GetServerDelayTimeBetweenHits))
  (if _returnvalue_2
    (Variables|Default|SetClassIndex 0)
    (if (> (Utilities|Array|Length (Class|MissionControlStorageManager|GetStoredObjectClasses (Variables|Default|GetMissionControlStorageManager))) 0)
      (Variables|Default|SetActiveClass (Utilities|Array|Get(acopy) (Class|MissionControlStorageManager|GetStoredObjectClasses (Variables|Default|GetMissionControlStorageManager))))
      (else
        (Variables|Default|SetActiveClass 0 :!label _label)))
    (else
      (goto _label)))
  (Class|MissionControlStorageManager|ServerSetIsOpen (Variables|Default|GetMissionControlStorageManager) _returnvalue_2))

(event EventBeginPlay
  (Utilities|FlowControl|Sequence
    (:then_0
      (if (not (Networking|IsDedicatedServer))
        ;[1 1 1] Client setup
        (Utilities|FlowControl|Sequence
          (:then_0
            (Class|MissionControlStorageManager|AddStorageLocation (Variables|Default|GetMissionControlStorageManager) (Variables|Default|GetStorageArea)))
          (:then_1
            (CallFunction|LocalUpdateOpenStatus))
          (:then_2
            (CallFunction|SpawnVisual))
          (:then_3
            (EventDispatchers|BindEventtoOnOpenStatusChanged (Variables|Default|GetMissionControlStorageManager) (EventDispatchers|CreateEvent :!event Custom|LocalUpdateOpenStatus))))))
    (:then_1
      (Networking|SwitchHasAuthority
        (:Authority
          ;[1 1 1] Bind on authority
          (EventDispatchers|BindEventtoOnInteract (Variables|Default|GetOpenSwitch) (EventDispatchers|CreateEvent :!event Custom|TapOpenToggle))
          (EventDispatchers|BindEventtoOnInteract (Variables|Default|GetLeftSelection) (EventDispatchers|CreateEvent :!event Custom|VRTapLeft))
          (EventDispatchers|BindEventtoOnInteract (Variables|Default|GetCenterSelection) (EventDispatchers|CreateEvent :!event Custom|VRTapCenter))
          (EventDispatchers|BindEventtoOnInteract (Variables|Default|GetRightSelection) (EventDispatchers|CreateEvent :!event Custom|VRTapRight)))))
    (:then_2
      (Rendering|Components|TextRender|SetText (Variables|Default|GetBoxName) (Variables|Default|GetStorageBoxName)))))

(fn ConstructionScript
  (|CallParentFunction)
  (Transformation|SetActorScale3D "1.000000,1.000000,1.000000")
  (bind _returnvalue (Rendering|Material|CreateDynamicMaterialInstance (Variables|Default|GetDebugSwitchVisualizer) 0 "/Game/Maps/Development/TempAssets/BluePrints/M_DebugSwitchColor.M_DebugSwitchColor" "None" :!class /Script/Engine.PrimitiveComponent))
  (Variables|Default|SetDebugSwitchMaterial _returnvalue))

(fn CanUse
  (params (InstigatorPawn :type Pawn%20Object%20Reference))
  (return (not (Class|MissionControlStorageManager|GetIsOpen (Variables|Default|GetMissionControlStorageManager)))))

(fn UpdateMenuVisuals
  (params (bShowBoxes :type Boolean))
  (Collision|SetCollisionEnabled (Variables|Default|GetLeftSelection) (select bShowBoxes "QueryOnly" "NoCollision"))
  (Rendering|SetVisibility (Variables|Default|GetDebugSwitchVisualizer1) bShowBoxes false))

(fn ClampIndex
  (params (NewIndex :type Integer))
  (bind _missioncontrolstoragemanager (Variables|Default|GetMissionControlStorageManager))
  (bind _returnvalue (Class|MissionControlStorageManager|GetStoredObjectClasses _missioncontrolstoragemanager))
  (bind _returnvalue_2 (Utilities|Array|Length _returnvalue))
  (if (< NewIndex 0)
    (return (- _returnvalue_2 1))
    (elif (>= NewIndex _returnvalue_2)
      (return 0)
      (else
        (return NewIndex)))))

(fn SpawnVisual
  (bind _visualspawn (Variables|Default|GetVisualSpawn))
  (bind _activeclass (Variables|Default|GetActiveClass))
  (bind _returnvalue (Transformation|GetWorldTransform _visualspawn))
  ;[1 0.01646 0] Just a temporary interface, no MP support
  (if (Utilities|IsValidClass _activeclass)
    (Utilities|FlowControl|Sequence
      (:then_0
        (Utilities|IsValid (Variables|Default|GetActiveSelection) :!label _label
          (:Is%20Valid
            (Actor|DestroyActor (Variables|Default|GetActiveSelection)))))
      (:then_1
        (bind _returnvalue_2 (|SpawnTempVisual _activeclass _returnvalue))
        (bind _output_get (Variables|Default|SetActiveSelection _returnvalue_2))
        (Transformation|AttachActorToActor _output_get self "None" "KeepRelative" "KeepRelative" "KeepRelative" true)
        (Utilities|FlowControl|Sequence
          (:then_0
            (bind _asmars_2030carryable_base (Utilities|Casting|CastToMars2030CarryableBase _returnvalue_2))
            (Collision|SetCollisionEnabled (Variables|/Script/MissionControl.Mars2030Interactable|GetMeshComponent _asmars_2030carryable_base) "NoCollision")
            (Utilities|IsValid (Actor|GetComponentbyClass _asmars_2030carryable_base "/Script/MissionControl.Mars2030FrobComponent")
              (:Is%20Valid
                (Collision|SetCollisionEnabled (Actor|GetComponentbyClass _asmars_2030carryable_base "/Script/MissionControl.Mars2030FrobComponent") "NoCollision"))))
          (:then_1
            (Transformation|SetActorTransform (Variables|Default|GetActiveSelection) _returnvalue)))))
    (else
      (goto _label))))

(fn OnRepClassIndex
  (CallFunction|SpawnVisual))

(fn OnRepNewVar1)

(fn OnRepActiveClass
  (CallFunction|SpawnVisual))
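; Hesperian boulder pickup for rock sample collection that breaks off a scannable rock after repeated hammer strikes.
; The server binds the specimen mesh's begin-overlap and accepts only components tagged RockSmasher.
; Each accepted hit calls HitRock to play a random impact sound at the sweep location and increments a hit counter.
; After six hits the counter resets and a BP_ScanableRock spawns at the Arrow's location.
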(event Custom|OnHammerRock
  (params (OverlappedComponent :type Primitive%20Component%20Object%20Reference) (OtherActor :type Actor%20Object%20Reference) (OtherComp :type Primitive%20Component%20Object%20Reference) (OtherBodyIndex :type Integer) (bFromSweep :type Boolean) (SweepResult :type Hit%20Result%20Structure%20%28by%20ref%29))
  (|CheckIsRockSmasher OtherComp
    (:then
      (CallFunction|HitRock (.Location (Collision|BreakHitResult SweepResult)) (Math|Random|RandomIntegerinRange 0 (- (Utilities|Array|Length (Variables|Default|GetRockHitSamples)) 1)))
      ;[1 1 1] Decrease count until 6 hits
      (bind _result (Math|Integer|IncrementInt (Variables|Default|GetRep_HitCounter))
        (:%20%20
          (if (> _result 5)
            ;[1 1 1] Spawn a rock
            (Variables|Default|SetRep_HitCounter 0) ; Reset counter
            (Game|SpawnActorfromClass "/Game/XRF/BP_ScanableRock.BP_ScanableRock_C" (Math|Transform|MakeTransform (Transformation|GetWorldLocation (Variables|Default|GetArrow)) "0, 0, 0" "1.000000,1.000000,1.000000") "AlwaysSpawn" 0 0)))))))

(event Custom|HitRock
  (params (Location :type Vector) (Sound :type Integer))
  ;[1 1 1] Client sound
  (Audio|SpawnSoundatLocation (Utilities|Array|Get(acopy) (Variables|Default|GetRockHitSamples) (Math|Integer|Clamp(Integer) Sound 0 (- (Utilities|Array|Length (Variables|Default|GetRockHitSamples)) 1))) Location "0, 0, 0" 1.0 1.0 0.0 0 0))

(event EventBeginPlay
  (|CallParentFunction)
  ;[1 1 1] Assign event on server
  (Networking|SwitchHasAuthority
    (:Authority
      (Collision|AssignOnComponentBeginOverlap (Variables|Default|GetSM_Specimen_2_Historcal_overlap) (EventDispatchers|CreateEvent :!event Custom|OnHammerRock)))))

(fn ConstructionScript
  (|CallParentFunction))
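; Cable actor for the EVA science deploy connection system, tracking which actor each of its ends is connected to.
; Authority-only setup and connection fill index-matched end and connection arrays with empty OnReps; connecting disables the end's collision and attaches it to the target point.
; Disconnect clears the entry and restores collision without detaching or checking authority.
; State queries fall back to the end's own state; HasAConnection always returns false.
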(fn ConstructionScript)

(fn OnRepCableEnds)

(fn OnRepCableConnections)

(fn SetCableEnds
  (params (NewCableEnds :type Array%20of%20BP%20Cable%20End%20Object%20References))
  (Networking|SwitchHasAuthority
    (:Authority
      (Variables|Default|SetCableEnds NewCableEnds))
    (:Remote
      (Development|PrintString "Cannot set cables from non authority"))))

(fn Connect
  (params (ActorNeedsConnection :type Actor%20Object%20Reference) (ConnectionPoint :type Scene%20Component%20Object%20Reference) (ConnectionPointOnSelf :type BP%20Cable%20End%20Object%20Reference))
  (Networking|SwitchHasAuthority
    (:Authority
      (bind _output_get (LocalVariables|SetFoundIndex (Utilities|Array|FindItem (Variables|Default|GetCableEnds) ConnectionPointOnSelf)))
      (if (>= _output_get 0)
        (Utilities|Array|SetArrayElem (Variables|Default|GetCableConnections) (LocalVariables|GetFoundIndex) ActorNeedsConnection)
        (Collision|SetCollisionEnabled (Variables|/Script/MissionControl.Mars2030Interactable|GetMeshComponent ConnectionPointOnSelf) "NoCollision")
        (Transformation|AttachComponentToComponent ConnectionPointOnSelf ConnectionPoint "None" "KeepWorld" "KeepWorld" "KeepWorld" true)
        (Transformation|SetActorRelativeTransform ConnectionPointOnSelf (Math|Transform|MakeTransform "0.000000,-3.000000, 0" "0, 0, 0" (Transformation|GetActorScale3D ConnectionPointOnSelf)) false false)
        (return true)
        (else
          (return false))))
    (:Remote
      (Development|PrintString "Cannont connect on non-authority"))))

(fn Disconnect
  (params (CableEnd :type BP%20Cable%20End%20Object%20Reference))
  (bind _cableconnections (Variables|Default|GetCableConnections))
  (bind _output_get (LocalVariables|SetFoundIndex (Utilities|Array|FindItem (Variables|Default|GetCableEnds) CableEnd)))
  (if (>= _output_get 0)
    (Utilities|IsValid (Utilities|Array|Get(acopy) _cableconnections (LocalVariables|GetFoundIndex))
      (:Is%20Valid
        (Utilities|Array|SetArrayElem _cableconnections (LocalVariables|GetFoundIndex) 0)
        (Collision|SetCollisionEnabled (Variables|/Script/MissionControl.Mars2030Interactable|GetMeshComponent CableEnd) "QueryAndPhysics")
        (return true))
      (:Is%20Not%20Valid
        _)))
  (return false))

(fn GetConnectedActors
  (return (Variables|Default|GetCableConnections)))

(fn GetConnectionState
  (params (ConnectionFromSelf :type BP%20Cable%20End%20Object%20Reference))
  (bind _cableends (Variables|Default|GetCableEnds))
  (bind _returnvalue (Utilities|Array|FindItem _cableends ConnectionFromSelf))
  (if (>= _returnvalue 0)
    (Utilities|IsValid (Utilities|Array|Get(acopy) (Variables|Default|GetCableConnections) _returnvalue)
      (:Is%20Valid
        (return "NewEnumerator3"))
      (:Is%20Not%20Valid
        (bind _newparam (Default|GetState ConnectionFromSelf))
        (return _newparam)))))

(fn HasAConnection
  (params (ConnectionPoint :type BP%20Cable%20End%20Object%20Reference))
  (return false))
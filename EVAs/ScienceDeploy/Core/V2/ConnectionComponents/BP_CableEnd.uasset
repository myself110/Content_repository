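; BP_CableEnd is a carryable end of a cable that plugs into connection points.
; On BeginPlay, the server's first end spawns a second end and a shared BP_Cable, then links all three.
; Grabbing disconnects the end through the cable, while dropping picks the closest overlapping BP_ConnectionPoint and asks the cable to connect it.
; GetState derives an enum state from the cable connection and carried flag.
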(event EventBeginPlay
  (bind _returnvalue (Transformation|GetActorTransform))
  (Networking|SwitchHasAuthority
    (:Authority
      (if (not (Variables|Spawn|GetbIsSecondEnd))
        (bind _returnvalue_2 (Game|SpawnActorfromClass "BP_CableEnd_C" (Math|Transform|MakeTransform (+ (.location _returnvalue) "-20.000000,0,0") (.rotation _returnvalue) (.scale _returnvalue)) "AdjustIfPossibleButAlwaysSpawn" 0 true 0))
        (bind _returnvalue_3 (Game|SpawnActorfromClass "/Game/EVAs/ScienceDeploy/Core/V2/ConnectionComponents/BP_Cable.BP_Cable_C" (Math|Transform|MakeTransform (.location _returnvalue) (.rotation _returnvalue) (.scale _returnvalue)) "AlwaysSpawn" 0 0))
        (Variables|Default|SetCableParent _returnvalue_3)
        (Variables|BP_CableEnd_C|SetCableParent _returnvalue_2 _returnvalue_3)
        (Default|SetCableEnds _returnvalue_3 (Utilities|Array|MakeArray self _returnvalue_2))))))

(event EventOnPostServerGrabbed
  (CallFunction|SetIsCarried true))

(event EventOnPostServerDrop
  (CallFunction|SetIsCarried false))

(fn ConstructionScript)

(fn IsBeingCarried
  (return (Variables|Default|GetbIsCarried)))

(fn OnRepBIsCarried)

(fn SetIsCarried
  (params (IsCarried :type Boolean))
  (bind _cableparent (Variables|Default|GetCableParent))
  (Variables|Default|SetbLastIsCarried (Variables|Default|GetbIsCarried))
  (bind _output_get (Variables|Default|SetbIsCarried IsCarried))
  (Networking|SwitchHasAuthority
    (:Authority
      (if _output_get
        (Utilities|IsValid _cableparent
          (:Is%20Valid
            (Class|BPIPDConnector|Disconnect(Message) _cableparent self)))
        (else
          (for _array_element (Class|PrimitiveComponent|GetOverlappingComponents (Variables|Default|GetCableOverlapPoint))
            ;[1 1 1] todo: check if already connected?
            (bind _asbp_connection_point (Utilities|Casting|CastToBP_ConnectionPoint _array_element))
            (Utilities|IsValid (LocalVariables|GetClosestPoint)
              (:Is%20Valid
                (if (|IsClosestPointVarFartherAway _asbp_connection_point (LocalVariables|GetClosestPoint))
                  (LocalVariables|SetClosestPoint _asbp_connection_point)))
              (:Is%20Not%20Valid
                (LocalVariables|SetClosestPoint _asbp_connection_point))))
          (Utilities|IsValid (LocalVariables|GetClosestPoint)
            (:Is%20Valid
              (Class|BPIPDConnector|Connect(Message) (Variables|Default|GetCableParent) (Components|GetOwner (LocalVariables|GetClosestPoint)) (LocalVariables|GetClosestPoint) self)
              (Development|PrintString "BP_CableEnd Connect"))))))))

(fn GetState
  (bind _cableparent (Variables|Default|GetCableParent))
  (Utilities|IsValid _cableparent
    (:Is%20Valid
      (bind _bhasconnection (Default|HasAConnection _cableparent self))
      (if _bhasconnection
        (return "NewEnumerator3")
        (else
          _)))
    (:Is%20Not%20Valid
      _))
  (if (== (Variables|Default|GetbIsCarried) true)
    (return "NewEnumerator1")
    (else
      (return "NewEnumerator0"))))

(fn OnRepCableParent)
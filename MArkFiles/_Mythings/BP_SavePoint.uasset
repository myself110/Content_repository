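; BP_SavePoint is an actor that prints a simulated radiation readout based on the player's distance, with no save logic despite its name.
; A timeline started on BeginPlay re-measures each update against the first BP_SavePoint found by GetActorOfClass, rather than Self.
; Within 1000 units it prints a random value around the low 50s.
; Out to 5000 units the value rises with distance plus random jitter; beyond that nothing prints.
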(event EventBeginPlay
  (Timeline|Timeline_0 Play
    (:Update
      (bind _returnvalue (Actor|GetActorOfClass "BP_SavePoint_C"))
      (if (<= (Transformation|GetDistanceTo (Game|Player|GetPlayerPawn 0) _returnvalue) 1e+03)
        (Development|PrintString (Utilities|String|ToString(Text) (Utilities|Text|FormatText "distance less than 1000 radiation is {radiation}" (Math|Random|RandomFloatinRange 5e+01 55.0))))
        (elif (<= (Transformation|GetDistanceTo (Game|Player|GetPlayerPawn 0) _returnvalue) 5e+03)
          (Development|PrintString (Utilities|String|ToString(Text) (Utilities|Text|FormatText "distance less than 5000 radiation is {radiation}" (+ (+ (/ (Transformation|GetDistanceTo (Game|Player|GetPlayerPawn 0) _returnvalue) 1e+02) 5e+01) (Math|Random|RandomFloatinRange 0.0 5.0))))))))))

(fn ConstructionScript)
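; Waypoint component that shows its owning character a navmesh route to an objective actor or location.
; The server finds the path, optionally repeating on a looping timer, and sends the points to the owning client to rebuild the supplied spline.
; Depending on NavMode, it either spaces reusable BP_WaypointActors along the spline, with an optional count cap, or has the owner add spline meshes per segment.
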(event Custom|FinishFindingWaypoint
  ;[1 1 1] Should be called when the player reach the objective. This will remove all waypoints created and clears the timer. @See BP_ObjectiveActor
  (Utilities|FlowControl|Sequence
    (:then_0
      (Variables|Waypoint|Private|SetGoalActor 0)
      (if (Variables|Waypoint|GetbDrawDebugStrings)
        (Class|KismetSystemLibrary|FlushDebugStrings)))
    (:then_1
      (Utilities|Time|ClearandInvalidateTimerbyHandle (Variables|Waypoint|Private|GetTimerHandle_FindPathToActor))
      (Utilities|ClearOutCachedActors)
      (CallFunction|InternalRemoveSplineMeshes))))

(event Custom|ServerFindPathToActor
  (params (GoalActor :type Actor%20Object%20Reference) (SplineComp :type Spline%20Component%20Object%20Reference))
  ;[1 0.06 0.06] Server will find path to actor. DO NOT call this directly from any other Blueprint. Instead call FindPathToActor event.
  (Variables|Waypoint|Private|SetGoalActor GoalActor)
  (Variables|Default|SetSplineComp SplineComp)
  (Variables|Waypoint|Private|SetGoalLocation "0, 0, 0")
  (CallFunction|InternalStartFindingPathtoActor)
  (CallFunction|InternalTryStartTimer))

(event Custom|ServerFindPathToLocation
  (params (GoalLocation :type Vector) (SplineComp :type Spline%20Component%20Object%20Reference))
  ;[1 0.06 0.06] Server will find path to location. DO NOT call this directly from any other Blueprint. Instead call FindPathToLocation event.
  (Variables|Waypoint|Private|SetGoalLocation GoalLocation)
  (Variables|Default|SetSplineComp SplineComp)
  (Variables|Waypoint|Private|SetGoalActor 0)
  (CallFunction|InternalStartFindingPathtoLocation)
  (CallFunction|InternalTryStartTimer))

(event Custom|FindPathToActor
  (params (Actor :type Actor%20Object%20Reference) (SplineComponent :type Spline%20Component%20Object%20Reference))
  ;[1 1 1] Sets the goal actor and spline component and starts finding path
  (Variables|Default|SetSplineComp SplineComponent)
  (Utilities|FlowControl|Sequence
    (:then_0
      (Spline|ClearSplinePoints (Variables|Default|GetSplineComp) true))
    (:then_1
      (CallFunction|ServerFindPathtoActor Actor (Variables|Default|GetSplineComp)))))

(event Custom|ClientPathFind
  (params (PathPoints :type Array%20of%20Vectors))
  (bind _splinecomp (Variables|Default|GetSplineComp))
  ;[1 1 1] This event will only execute on the owning client (that means the client who requested the server find path function)
  (Spline|ClearSplinePoints (Variables|Default|GetSplineComp) true)
  (for (_array_element _array_index) PathPoints
    (Spline|AddSplinePoint _splinecomp _array_element "World" true)
    (Spline|SetSplinePointType _splinecomp _array_index "CurveClamped" true))
  (switch Utilities|FlowControl|Switch|SwitchonENavMode (Variables|Waypoint|GetNavMode)
    (:NewEnumerator0
      (CallFunction|InternalPathFindingSpawnMode))
    (:NewEnumerator1
      (CallFunction|InternalPathFindingSplineMode))))

(event Custom|FindPathToLocation
  (params (Location :type Vector) (SplineComponent :type Spline%20Component%20Object%20Reference))
  ;[1 1 1] Sets the goal location and spline component and starts finding path
  (bind _output_get (Variables|Default|SetSplineComp SplineComponent))
  (CallFunction|ServerFindPathtoLocation Location _output_get))

(fn SetEnableWaypoint
  (params (bEnableWaypoint :type Boolean))
  ;[1 1 1] Set to true to enable this waypoint
  (Variables|Waypoint|Private|SetbEnableWaypoint bEnableWaypoint))

(fn IsWaypointEnabled
  ;[1 1 1] Returns true of this waypoint is enabled
  (return (Variables|Waypoint|Private|GetbEnableWaypoint)))

(fn GetGoalActor
  ;[1 1 1] Returns the objective Actor
  (return (Variables|Waypoint|Private|GetGoalActor)))

(fn InternalStartFindingPathtoActor
  (bind _returnvalue (Components|GetOwner))
  (Utilities|FlowControl|Sequence
    (:then_0
      ;[1 1 1] If the user chose to show debug strings then we remove all the previous strings
      (if (Variables|Waypoint|GetbDrawDebugStrings)
        (Class|KismetSystemLibrary|FlushDebugStrings)))
    (:then_1
      ;[1 1 1] Here we fist check if this waypoint is enabled. If it is then we make sure Goal Actor and Spline Comp (from Character) are valid. In case if the Goal Actor or Spline Comp are not valid, we set the appropriate Error Message so we know why this function didnt finish properly
      (if (Variables|Waypoint|Private|GetbEnableWaypoint)
        (Utilities|IsValid (Variables|Waypoint|Private|GetGoalActor)
          (:Is%20Valid
            (Utilities|IsValid (Variables|Default|GetSplineComp)
              (:Is%20Valid
                ;[1 1 1] This is our main function that finds the path (route) from Owner (which will be the Character that we added this component to) location to objective actor.
                (bind _returnvalue_2 (Class|NavigationSystemV1|FindPathtoActorSynchronously (Transformation|GetActorLocation _returnvalue) (Variables|Waypoint|Private|GetGoalActor) 5e+01 _returnvalue (Variables|Waypoint|GetNavFilterClass)))
                (if (Utilities|IsValid _returnvalue_2)
                  (CallFunction|ClientPathFind (Variables|/Script/NavigationSystem.NavigationPath|GetPathPoints _returnvalue_2))
                  (else
                    (LocalVariables|SetLocal_ErrorMessage "No Nav path found. Do you have Nav Mesh in world? Or are you in air?"))))
              (:Is%20Not%20Valid
                (LocalVariables|SetLocal_ErrorMessage "No spline component found"))))
          (:Is%20Not%20Valid
            (LocalVariables|SetLocal_ErrorMessage "Goal Actor is invalid")))
        (else
          (LocalVariables|SetLocal_ErrorMessage "Waypoint not enabled"))))
    (:then_2
      ;[1 1 1] When this function finishes execution, it will check if we faced any errors. If any errors then print that out to the user.
      (if (not (Utilities|Text|TextIsEmpty (LocalVariables|GetLocal_ErrorMessage)))
        (bind _output_get (LocalVariables|SetLocal_FormatErrorMessage (Utilities|Text|FormatText "WAYPOINT ERROR: {Message}" (LocalVariables|GetLocal_ErrorMessage))))
        (Development|PrintText _output_get true true "(R=1.000000,G=0.038198,B=0.009546,A=1.000000)" 1e+01)))))

(fn InternalTryStartTimer
  ;[1 1 1] If the Tick Time is greater than 0 then we create a new timer that calls StartFindingPath function at given intervals
  (if (> (Variables|Waypoint|GetTickTime) 0.0)
    (bind _returnvalue (Utilities|Time|SetTimerbyEvent (EventDispatchers|CreateEvent :!event InternalStartPathFinding) (Variables|Waypoint|GetTickTime) true))
    (Variables|Waypoint|Private|SetTimerHandle_FindPathToActor _returnvalue)))

(fn InternalPathFindingSplineMode
  (bind _splinecomp (Variables|Default|GetSplineComp))
  (CallFunction|InternalRemoveSplineMeshes)
  ;[1 1 1] In this for loop we set the last index to the total points of spline - 2. This is to avoid getting the first and last points.
  (for _index (range 0 (- (Spline|GetNumberOfSplinePoints (Variables|Default|GetSplineComp)) 2))
    (bind _returnvalue (Class|BPIWaypoint|AddWaypointSplineComponent(Message) (Components|GetOwner)))
    ;[1 1 1] As the for loop iterates through each points, we add a new spline component and add it to spline mesh components array. We also get the location of that specific index and next index (by adding 1 to it) and use that information to set the Start and End points of added spline
    (Utilities|Array|Add (Variables|Waypoint|Private|GetAddedSplineMeshComponents) _returnvalue)
    (SplineMesh|SetStartandEnd _returnvalue (.Location (Spline|GetLocationandTangentatSplinePoint _splinecomp _index "World")) (.Tangent (Spline|GetLocationandTangentatSplinePoint _splinecomp _index "World")) (.Location (Spline|GetLocationandTangentatSplinePoint _splinecomp (+ _index 1) "World")) (.Tangent (Spline|GetLocationandTangentatSplinePoint _splinecomp (+ _index 1) "World")) true :!class /Script/Engine.SplineMeshComponent)))

(fn InternalPathFindingSpawnMode
  (LocalVariables|SetbLocal_SpawningIsClamped (> (Variables|Waypoint|GetMaxNumberOfMeshes) 0))
  (Utilities|FlowControl|Sequence
    (:then_0
      ;[1 1 1] Sets the number of meshes to spawn based on the distance to objective and distance allowed between each mesh. We clamp that value to Max Number of Meshes to make sure we dont spawn too much
      (Variables|Waypoint|Private|SetMeshesToSpawn (Math|Float|Truncate (/ (Spline|GetSplineLength (Variables|Default|GetSplineComp)) (* (Variables|Waypoint|GetMeshDistance) 2.0))))
      (if (LocalVariables|GetbLocal_SpawningIsClamped)
        (Variables|Waypoint|Private|SetMeshesToSpawn (Math|Integer|Clamp(Integer) (Variables|Waypoint|Private|GetMeshesToSpawn) 0 (Variables|Waypoint|GetMaxNumberOfMeshes)))))
    (:then_1
      ;[1 1 1] Once the number of Meshes to Spawn is set, we do a for loop from index 1. This is because we dont want waypoint mesh to spawn at character location.
      (LocalVariables|SetLocal_Point (/ (Spline|GetSplineLength (Variables|Default|GetSplineComp)) (Math|Conversions|ToFloat(Integer) (Variables|Waypoint|Private|GetMeshesToSpawn))))
      (Utilities|FlowControl|Sequence
        (:then_0
          (if (LocalVariables|GetbLocal_SpawningIsClamped)
            ;[1 1 1] Check if there are any changes and only proceed if any change.
            (if (!= (Utilities|Array|Length (Variables|Waypoint|Private|GetSpawnedMeshes)) (Variables|Waypoint|Private|GetMeshesToSpawn))
              (Utilities|ClearOutCachedActors))))
        (:then_1
          (if (LocalVariables|GetbLocal_SpawningIsClamped)
            (Utilities|UpdateLocationOfCachedActors (LocalVariables|GetLocal_Point)
              (:NotUpdated
                (Utilities|RefreshCachedActors (LocalVariables|GetLocal_Point) :!label _label)))
            (elif (!= (Utilities|Array|Length (Variables|Waypoint|Private|GetSpawnedMeshes)) (Variables|Waypoint|Private|GetMeshesToSpawn))
              (goto _label)
              (else
                (Utilities|UpdateLocationOfCachedActors (LocalVariables|GetLocal_Point))))))))))

(fn InternalStartFindingPathtoLocation
  (bind _returnvalue (Components|GetOwner))
  (Utilities|FlowControl|Sequence
    (:then_0
      ;[1 1 1] If the user chose to show debug strings then we remove all the previous strings
      (if (Variables|Waypoint|GetbDrawDebugStrings)
        (Class|KismetSystemLibrary|FlushDebugStrings)))
    (:then_1
      ;[1 1 1] Here we fist check if this waypoint is enabled. If it is then we make sure Spline Comp (from Character) is valid. If it is we clear all spline points previously created so we can create new spline points.
      ; In case if the Spline Comp was not valid, we set the appropriate Error Message so we know why this function didnt finish properly.
      (if (Variables|Waypoint|Private|GetbEnableWaypoint)
        (Utilities|IsValid (Variables|Default|GetSplineComp)
          (:Is%20Valid
            (Spline|ClearSplinePoints (Variables|Default|GetSplineComp) true)
            ;[1 1 1] This is our main function that finds the path (route) from Owner (which will be the Character that we added this component to) location to objective location.
            (bind _returnvalue_2 (Class|NavigationSystemV1|FindPathtoLocationSynchronously (Transformation|GetActorLocation _returnvalue) (Variables|Waypoint|Private|GetGoalLocation) _returnvalue (Variables|Waypoint|GetNavFilterClass)))
            (if (Utilities|IsValid _returnvalue_2)
              (CallFunction|ClientPathFind (Variables|/Script/NavigationSystem.NavigationPath|GetPathPoints _returnvalue_2))
              (else
                (LocalVariables|SetLocal_ErrorMessage "No Nav path found. Do you have Nav Mesh in world? Or are you in air?"))))
          (:Is%20Not%20Valid
            (LocalVariables|SetLocal_ErrorMessage "No spline component found")))
        (else
          (LocalVariables|SetLocal_ErrorMessage "Waypoint not enabled"))))
    (:then_2
      ;[1 1 1] When this function finishes execution, it will check if we faced any errors. If any errors then print that out to the user.
      (if (not (Utilities|Text|TextIsEmpty (LocalVariables|GetLocal_ErrorMessage)))
        (bind _output_get (LocalVariables|SetLocal_FormatErrorMessage (Utilities|Text|FormatText "WAYPOINT ERROR: {Message}" (LocalVariables|GetLocal_ErrorMessage))))
        (Development|PrintText _output_get true true "(R=1.000000,G=0.038198,B=0.009546,A=1.000000)" 1e+01)))))

(fn InternalRemoveSplineMeshes
  (bind _addedsplinemeshcomponents (Variables|Waypoint|Private|GetAddedSplineMeshComponents))
  (Class|BPIWaypoint|RemoveSplineMeshes(Message) (Components|GetOwner) _addedsplinemeshcomponents)
  (Utilities|Array|Clear _addedsplinemeshcomponents))

(fn InternalStartPathFinding
  (Utilities|IsValid (Variables|Waypoint|Private|GetGoalActor)
    (:Is%20Valid
      (CallFunction|InternalStartFindingPathtoActor))
    (:Is%20Not%20Valid
      (CallFunction|InternalStartFindingPathtoLocation))))